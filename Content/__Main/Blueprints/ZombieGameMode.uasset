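; Game mode for a zombie wave-survival game that runs waves until the player wins after the final one.
; Each wave spawns an ammo crate at a random preset location and a zombie count scaled by wave number, split between two spawn points.
; ZombieKilled counts down remaining zombies, then either triggers the win UI or shows the next wave's UI and spawns it after a delay.
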(event `self.ReceiveBeginPlay`
  ;[1 1 1] Start Game
  (`self.StartGame`))

(event `StartGame`
  ;[1 1 1] Start Game
  (`self.Spawn Zombies`))

(event `Spawn Zombies`
  ;[1 1 1] Spawn Zombies
  (`self.Spawn Ammo`)
  (bind _output_get (set `self.ZombieTotal` (* (`self.CurrentWave`) 4)))
  (set `self.ZombiesLeft` _output_get)
  (for _index (range (+ _output_get 1))
    (if (== _index (/ (`self.ZombieTotal`) 2))
      (break)
      (else
        (`|SpawnActorFromClass` "/Game/__Main/Zombie/BP_zombie.BP_zombie_C" (`self.Spawn Location 1`) "Undefined" "MultiplyWithRoot" null null))))
  (for _ (range 1 (+ (/ (`self.ZombieTotal`) 2) 1))
    (`|SpawnActorFromClass` "/Game/__Main/Zombie/BP_zombie.BP_zombie_C" (`self.Spawn Location 2`) "Undefined" "MultiplyWithRoot" null null)))

(event `Zombie Killed`
  ;[1 1 1] Zombie Killed
  (bind _result (`/Engine/EditorBlueprintResources/StandardMacros.DecrementInt` (`self.ZombiesLeft`))
    (:`  `
      (if (== _result 0)
        (`self.Wave Increment`)))))

(event `Wave Start`
  ;[1 1 1] Start Next Wave
  (bind _asbp_first_person_character (cast `/Game/__Main/Blueprints/BP_FirstPersonCharacter` (`GameplayStatics.GetPlayerCharacter` 0)))
  (`/Game/__Main/Blueprints/BP_FirstPersonCharacter.Show Wave UI` _asbp_first_person_character (`self.CurrentWave`))
  (`KismetSystemLibrary.Delay` 5.0)
  (`self.Spawn Zombies`))

(event `Wave Increment`
  ;[1 1 1] Wave System
  (if (== (`self.CurrentWave`) (`self.MaxWaves`))
    (`self.Player Wins`)
    (else
      (`/Engine/EditorBlueprintResources/StandardMacros.IncrementInt` (`self.CurrentWave`)
        (:`  `
          (`self.Wave Start`))))))

(event `Player Wins`
  ;[1 1 1] Win Logic
  (`KismetSystemLibrary.LogString` "You won the game")
  (bind _asbp_first_person_character (cast `/Game/__Main/Blueprints/BP_FirstPersonCharacter` (`GameplayStatics.GetPlayerCharacter` 0)))
  (`/Game/__Main/Blueprints/BP_FirstPersonCharacter.Show Win UI` _asbp_first_person_character))

(event `Spawn Ammo`
  ;[1 1 1] Spawn Ammo Crate
  (`|SpawnActorFromClass` "/Game/__Main/Blueprints/BP_AmmoCrate.BP_AmmoCrate_C" (`KismetMathLibrary.MakeTransform` (`|GetArrayItem` (`self.AmmoCrateLocations`) (`KismetMathLibrary.RandomInteger` 3))) "Undefined" "MultiplyWithRoot" null null))

(fn `UserConstructionScript`)